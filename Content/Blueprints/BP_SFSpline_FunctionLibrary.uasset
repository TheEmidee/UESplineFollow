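; Blueprint function library of helpers for SFSpline markers and distances along a spline.
; It checks whether a marker's object matches a class and converts between world and normalized distances, clamped to the spline's range.
; A nested-loop swap sort orders marker actors by normalized start distance, read from either the single action point or window start depending on marker type.
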(fn `GetDistanceSortedMarkerActors`
  (params (MarkerActors :type "Array of /SplineFollow/Blueprints/BP_SplineMarker Object Reference"))
  (returns (SortedMarkers :type "Array of /SplineFollow/Blueprints/BP_SplineMarker Object Reference"))
  (locals (Markers :type "Array of /SplineFollow/Blueprints/BP_SplineMarker Object Reference"))
  (bind _output_get (set `local.Markers` MarkerActors))
  (for (_array_element _array_index) _output_get
    (for _index (range (+ (`KismetArrayLibrary.Array_LastIndex` _output_get) 1))
      (if (> (`self.GetStartNormalizedDistance` (`/SplineFollow/Blueprints/BP_SplineMarker.SplineMarker` (`|GetArrayItem` (`local.Markers`) _index))) (`self.GetStartNormalizedDistance` (`/SplineFollow/Blueprints/BP_SplineMarker.SplineMarker` _array_element)))
        (`KismetArrayLibrary.Array_Swap` (`local.Markers`) _index _array_index))))
  (return (`local.Markers`)))

(fn `GetStartNormalizedDistance`
  (params (SFSplineMarker :type "SFSplineMarker Structure (by ref)"))
  (returns (ReturnValue :type "Float (single-precision)"))
  (bind ((`Type` _type) (`SingleActionNormalizedSplineDistance` _singleactionnormalizedsplinedistance) (`WindowStartNormalizedSplineDistance` _windowstartnormalizedsplinedistance)) (break `SFSplineMarkerInfos` (`.Infos` (break `SFSplineMarker` SFSplineMarker))))
  (return (select `ESFSplineMarkerType` _type :`Single` _singleactionnormalizedsplinedistance :`Window` _windowstartnormalizedsplinedistance)))

(fn `IsMarkerOfType`
  (params (SFSplineMarker :type "SFSplineMarker Structure (by ref)") (ObjectClass :type "Object Class Reference"))
  (returns (ReturnValue :type Boolean))
  (bind ((`Object` _object)) (break `SFSplineMarker` SFSplineMarker))
  (return (and (`KismetSystemLibrary.IsValid` _object) (or (`GameplayStatics.ObjectIsA` _object ObjectClass) (`KismetMathLibrary.ClassIsChildOf` (`GameplayStatics.GetObjectClass` _object) ObjectClass)))))

(fn `NormalizedDistanceToUnrealDistance`
  (params (NormalizedDistance :type "Float (single-precision)") (SplineLength :type "Float (double-precision)"))
  (returns (Distance :type "Float (double-precision)"))
  (return (`KismetMathLibrary.FClamp` (* NormalizedDistance SplineLength) 0.0 SplineLength)))

(fn `UnrealDistanceToNormalizedDistance`
  (params (Distance :type "Float (single-precision)") (SplineLength :type "Float (double-precision)"))
  (returns (NormalizedDistance :type "Float (double-precision)"))
  (return (`KismetMathLibrary.FClamp` (/ Distance SplineLength))))